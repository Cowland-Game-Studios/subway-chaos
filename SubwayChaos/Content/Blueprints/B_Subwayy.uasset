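; Clickable subway train actor that plays a horn in easter-egg mode or otherwise opens a details view.
; Setup colors head and tail lights by direction, writes the level name and a random train ID on its signs, and sets ProjectileMovement velocity.
; Outside easter-egg mode, hovering turns emitters from yellow to white with a sound.
; Clicking runs a delay-looped MoveObjectWidget transition from player pawn to train, then shows the widget.
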(event `self.ReceiveActorOnClicked`
  (params (ButtonPressed :type "Key Structure"))
  ;[1 1 1] easter egg
  (if (`self.IsEasterEggable`)
    (`GameplayStatics.PlaySoundAtLocation` "/Game/SoundFX/TrainHornMadeMyself.TrainHornMadeMyself" (`SceneComponent.K2_GetComponentLocation` (`self.Train`)) (struct) 1.0 1.0 0.0 null null null)
    (else
      (`GameplayStatics.PlaySound2D` "/Game/SoundFX/Clicked.Clicked" 1.0 1.0 0.0 null null)
      (`self.SubwayDetails`))))

(event `self.Train.OnBeginCursorOver`
  (params (TouchedComponent :type "PrimitiveComponent Object Reference"))
  ;[1 1 1] play sound at hover
  ;[1 1 1] easter egg
  (set `self.isOver` true)
  (if (not (`self.IsEasterEggable`))
    (`GameplayStatics.PlaySound2D` "/Game/SoundFX/Selection.Selection" 1.0 1.0 0.0 null null)
    (for _array_element (`|MakeArray` (`self.LightEmitter8`) (`self.LightEmitter1`) (`self.LightEmitter2`) (`self.LightEmitter3`) (`self.LightEmitter4`) (`self.LightEmitter5`) (`self.LightEmitter6`) (`self.LightEmitter7`) (`self.LightEmitter`) (`self.LightEmitter9`) (`self.LightEmitter10`) (`self.LightEmitter11`) (`self.LightEmitter12`) (`self.LightEmitter13`) (`self.LightEmitter15`) (`self.LightEmitter14`))
      (`LightComponent.SetLightColor` _array_element (struct :`R` 1.0 :`G` 1.0 :`B` 1.0 :`A` 1.0) true))))

(event `self.Train.OnEndCursorOver`
  (params (TouchedComponent :type "PrimitiveComponent Object Reference"))
  ;[1 1 1] play sound at hover
  (set `self.isOver` false)
  (if (not (`self.IsEasterEggable`))
    (for _array_element (`|MakeArray` (`self.LightEmitter8`) (`self.LightEmitter1`) (`self.LightEmitter2`) (`self.LightEmitter3`) (`self.LightEmitter4`) (`self.LightEmitter5`) (`self.LightEmitter6`) (`self.LightEmitter7`) (`self.LightEmitter`) (`self.LightEmitter9`) (`self.LightEmitter10`) (`self.LightEmitter11`) (`self.LightEmitter12`) (`self.LightEmitter13`) (`self.LightEmitter15`) (`self.LightEmitter14`))
      (`LightComponent.SetLightColor` _array_element (struct :`R` 1.0 :`G` 0.974143 :`A` 1.0) true))))

(event `self.ReceiveBeginPlay`
  ;[1 1 1] setup
  (`self.Setup` false))

(fn `Setup`
  (params (IsFlipped :type Boolean) (IsHead :type Boolean) (Velocity :type "Vector Structure"))
  (bind _array (`|MakeArray` (make `LinearColor` :`R` 255.0 :`G` 255.0 :`B` 255.0) (make `LinearColor` :`R` 255.0)))
  (bind _output (`|GetArrayItem` _array))
  (bind _output_2 (`|GetArrayItem` _array 1))
  ;[1 1 1] set dynamic lights and text
  (for _array_element (`|MakeArray` (`self.HeadLightFLB`) (`self.HeadLightFLT`) (`self.HeadLightFRB`) (`self.HeadLightFRT`))
    (if IsFlipped
      (`LightComponent.SetLightColor` _array_element _output_2 true)
      (else
        (`LightComponent.SetLightColor` _array_element _output true)))
    (if IsHead
      (`LightComponent.SetIntensity` _array_element 10000.0)))
  (for _array_element_2 (`|MakeArray` (`self.HeadLightBLB`) (`self.HeadLightBLT`) (`self.HeadLightBRB`) (`self.HeadLightBRT`))
    (if IsFlipped
      (`LightComponent.SetLightColor` _array_element_2 _output true)
      (else
        (`LightComponent.SetLightColor` _array_element_2 _output_2 true)))
    (if IsHead
      (`LightComponent.SetIntensity` _array_element_2 10000.0)))
  (for _array_element_3 (`|MakeArray` (`self.DestinationText_BR`) (`self.DestinationText_FR`) (`self.DestinationText_BL`) (`self.DestinationText_FL`))
    (bind _returnvalue (`GameplayStatics.GetCurrentLevelName` true))
    (`TextRenderComponent.K2_SetText` _array_element_3 (`KismetTextLibrary.Conv_StringToText` _returnvalue)))
  (bind _output_get (set `self.trainNumber` (`KismetMathLibrary.RandomIntegerInRange` 1000 9999)))
  (for _array_element_4 (`|MakeArray` (`self.TrainID_BL`) (`self.TrainID_FL`) (`self.TrainID_FR`) (`self.TrainID_BR`))
    (`TextRenderComponent.K2_SetText` _array_element_4 (`KismetTextLibrary.Conv_IntToText` _output_get false false)))
  (set `MovementComponent.Velocity` Velocity (`self.ProjectileMovement`)))

(fn `UserConstructionScript`)