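; Level spawner actor that continuously spawns B_Subwayy train actors, starting on BeginPlay and repeating after a configurable delay.
; Each spawn uses the TrainLocation transform with fixed world Y and Z offsets and always spawns regardless of collision.
; SetupSubway then passes the flip flag, head flag and speed to the new subway, negating the velocity when flipped.
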(event `self.ReceiveBeginPlay`
  (bind (_returnvalue_location_x _returnvalue_rotation _returnvalue _returnvalue2) (`self.GetPositions` :!label _label))
  (bind _returnvalue_2 (`|SpawnActorFromClass` "/Game/Blueprints/B_Subwayy.B_Subwayy_C" (`KismetMathLibrary.MakeTransform` (`KismetMathLibrary.MakeVector` _returnvalue_location_x _returnvalue2 _returnvalue) _returnvalue_rotation) "AlwaysSpawn" "OverrideRootScale" null null))
  (`self.SetupSubway` _returnvalue_2 _returnvalue_2)
  (`KismetSystemLibrary.Delay` (`self.Delay`))
  (goto _label))

(fn `GetPositions`
  (returns (ReturnValue_Location_X :type "Float (double-precision)") (ReturnValue_Rotation :type "Rotator Structure") (ReturnValue :type "Float (double-precision)") (ReturnValue2 :type "Float (double-precision)"))
  (bind _returnvalue (`SceneComponent.K2_GetComponentToWorld` (`self.Train Location`)))
  (return (.x (.location _returnvalue)) (.rotation _returnvalue) (+ (.z (.location _returnvalue)) 300.0) (+ (.y (.location _returnvalue)) 190.0)))

(fn `SetupSubway`
  (params (self2 :type "/Game/Blueprints/B_Subwayy Object Reference") (self3 :type "/Game/Blueprints/B_Subwayy Object Reference"))
  (bind _flip (`self.Flip`))
  (bind _speed (`self.Speed`))
  (bind _ishead (`self.IsHead`))
  (if _flip
    (`/Game/Blueprints/B_Subwayy.Setup` self2 _flip _ishead (* _speed -1.0))
    (else
      (`/Game/Blueprints/B_Subwayy.Setup` self3 _flip _ishead _speed))))

(fn `UserConstructionScript`)