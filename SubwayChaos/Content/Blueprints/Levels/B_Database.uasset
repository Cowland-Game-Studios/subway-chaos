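; B_Database is an actor that holds a level's train and game-over bookkeeping for a subway game.
; Construction passes the train counters to UpdateDataInt, a by-ref batch setter guarded by an IsWriting flag, to zero them, and sets the actor's rotation.
; Every Tick, IsGameOver compares the B_Subwayy actor count against the counters and only prints "game over".
; Per-level defaults and widget/camera-fade setup sit in unconnected nodes that never run.
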(event `self.ReceiveTick`
  (params (DeltaSeconds :type "Float (single-precision)"))
  (`self.IsGameOver`))

(fn `IsGameOver`
  (bind _outactors (`GameplayStatics.GetAllActorsOfClass` "/Game/Blueprints/Trains/B_Subwayy.B_Subwayy_C"))
  (if (and (== (`KismetArrayLibrary.Array_Length` _outactors) (- (- (`self.TrainsCrashed`) (`self.TrainsCleanedUp`)) (`self.TrainsRemaining`))) (== (`self.TrainsRemaining`) 0))
    (`KismetSystemLibrary.PrintString` "game over")))

(fn `UpdateDataInt`
  (params (Array :type "Array of Integer") (Value :type Integer))
  (returns (ReturnValue :type "EventReply Structure"))
  (if (not (`self.IsWriting`))
    (set `self.IsWriting` true)
    (for _array_element Array
      (`|VariableSetRef` _array_element Value))
    (set `self.IsWriting` false)
    (return (`WidgetBlueprintLibrary.Handled`))
    (else
      (return (`WidgetBlueprintLibrary.Unhandled`)))))

(fn `UserConstructionScript`
  (`self.UpdateDataInt` (`|MakeArray` (`self.TrainsPassed`) (`self.TrainsRemaining`) (`self.TrainsCrashed`) (`self.TrainsValidated`)))
  ;[1 1 1] when constructed, make the widget
  (`self.K2_SetActorRotation` (struct :`Pitch` -50.0 :`Yaw` 90.0)))