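; B_Subway is a subway train actor that dresses its lights and signage on BeginPlay.
; It sets front headlights white and rear ones red, as the RandomInteger(1) color pick always returns zero.
; It writes the current level name to the four destination texts and a random four-digit train number, stored in TrainNumber, to the four ID texts.
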(event `self.ReceiveBeginPlay`
  (bind _returnvalue (`KismetMathLibrary.RandomInteger` 1))
  (bind _array (`|MakeArray` (make `LinearColor` :`R` 255.0 :`G` 255.0 :`B` 255.0) (make `LinearColor` :`R` 255.0)))
  (for _array_element (`|MakeArray` (`self.HeadLightFLB`) (`self.HeadLightFLT`) (`self.HeadLightFRB`) (`self.HeadLightFRT`))
    (`LightComponent.SetLightColor` _array_element (`|GetArrayItem` _array _returnvalue) true))
  (for _array_element_2 (`|MakeArray` (`self.HeadLightBLB`) (`self.HeadLightBLT`) (`self.HeadLightBRB`) (`self.HeadLightBRT`))
    (`LightComponent.SetLightColor` _array_element_2 (`|GetArrayItem` _array (`KismetMathLibrary.Abs_Int` (- _returnvalue 1))) true))
  (for _array_element_3 (`|MakeArray` (`self.DestinationText_BR`) (`self.DestinationText_FR`) (`self.DestinationText_BL`) (`self.DestinationText_FL`))
    (bind _returnvalue_2 (`GameplayStatics.GetCurrentLevelName` true))
    (`TextRenderComponent.K2_SetText` _array_element_3 (`KismetTextLibrary.Conv_StringToText` _returnvalue_2)))
  (bind _output_get (set `self.trainNumber` (`KismetMathLibrary.RandomIntegerInRange` 1000 9999)))
  (for _array_element_4 (`|MakeArray` (`self.TrainID_BL`) (`self.TrainID_FL`) (`self.TrainID_FR`) (`self.TrainID_BR`))
    (`TextRenderComponent.K2_SetText` _array_element_4 (`KismetTextLibrary.Conv_IntToText` _output_get false false))))

(fn `UserConstructionScript`)