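; B_Subwayy is a clickable subway train that moves by projectile movement and can crash into other trains.
; Construction sets its lights, line letter and color, destination from level name and random car number.
; Hover highlights it and clicking moves the view to a paused details widget while near initial velocity; easter-egg trains just honk.
; Overlapping another train triggers a physics wreck with effects and database tally, which a click cleans up.
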(event `self.ReceiveActorOnClicked`
  (params (ButtonPressed :type "Key Structure"))
  (if (`self.IsEasterEggable`)
    ;[1 1 1] easter egg
    (`GameplayStatics.PlaySoundAtLocation` "/Game/SoundFX/train/TrainHornMadeMyself.TrainHornMadeMyself" (`SceneComponent.K2_GetComponentLocation` (`self.Train`)) (struct) 1.0 1.0 0.0 null null null)
    (elif (not (`self.IsDestroyed`))
      (if (`self.GetIsTrainSlow`)
        (`GameplayStatics.PlaySound2D` "/Game/SoundFX/ui/Clicked.Clicked" 1.0 1.0 0.0 null null)
        (`self.SubwayDetails`))
      (else
        (`self.CleanTrain`)))))

(event `self.Train.OnBeginCursorOver`
  (params (TouchedComponent :type "PrimitiveComponent Object Reference"))
  ;[1 1 1] play sound at hover
  (if (`self.GetIsTrainSlow`)
    (if (not (`self.IsEasterEggable`))
      (set `self.isMouseOver` true)
      (`GameplayStatics.PlaySound2D` "/Game/SoundFX/ui/Selection.Selection" 1.0 1.0 0.0 null null)
      (for _array_element (`self.MakeArrayOfLights`)
        (`LightComponent.SetLightColor` _array_element (struct :`R` 1.0 :`G` 1.0 :`B` 1.0 :`A` 1.0) true))
      (`PrimitiveComponent.SetMaterial` (`self.Inside_Filler`) 0 "/Game/Texture_Model/Materials/M_LitUpHovered.M_LitUpHovered"))))

(event `self.Train.OnEndCursorOver`
  (params (TouchedComponent :type "PrimitiveComponent Object Reference"))
  ;[1 1 1] play sound at hover
  (if (`self.GetIsTrainSlow`)
    (if (not (`self.IsEasterEggable`))
      (set `self.isMouseOver` false)
      (for _array_element (`self.MakeArrayOfLights`)
        (`LightComponent.SetLightColor` _array_element (struct :`R` 1.0 :`G` 0.974143 :`A` 1.0) true))
      (`PrimitiveComponent.SetMaterial` (`self.Inside_Filler`) 0 "/Game/Texture_Model/Materials/M_LitUp.M_LitUp"))))

(event `self.Hitbox.OnComponentBeginOverlap`
  (params (OverlappedComponent :type "PrimitiveComponent Object Reference") (OtherActor :type "Actor Object Reference") (OtherComp :type "PrimitiveComponent Object Reference") (OtherBodyIndex :type Integer) (bFromSweep :type Boolean) (SweepResult :type "HitResult Structure (by ref)"))
  (if (and (not (`self.IsEasterEggable`)) (== (`GameplayStatics.GetObjectClass` OtherActor) "B_Subwayy_C") (!= OtherActor self))
    (`/Engine/EditorBlueprintResources/StandardMacros.DoOnce` false
      (:`Completed`
        (`self.Crash`)))))

(fn `CleanTrain`
  (bind _outactors (`GameplayStatics.GetAllActorsOfClass` "/Game/Blueprints/Levels/B_Database.B_Database_C"))
  (`/Engine/EditorBlueprintResources/StandardMacros.IncrementInt` (`/Game/Blueprints/Levels/B_Database.TrainsCleanedUp` (`|GetArrayItem` _outactors))
    (:`  `
      (`self.K2_DestroyActor`))))

(fn `GetIsTrainSlow`
  (returns (ReturnValue :type Boolean))
  (return (== (`self.InitialVelocity`) (`MovementComponent.Velocity` (`self.ProjectileMovement`)) :`ErrorTolerance` 1.0)))

(fn `GetTrainColorByLetter`
  (params (ItemToFind :type "String (by ref)"))
  (returns (Output :type "LinearColor Structure (by ref)"))
  (bind _array (`|MakeArray` "1" "2" "3" "4" "5" "6" "7" "A" "B" "C" "D" "E" "F" "G" "J" "L" "M" "N" "Q" "R" "S" "V" "W" "Z"))
  (bind _returnvalue (`KismetArrayLibrary.Array_Find` _array ItemToFind))
  (if (!= _returnvalue -1)
    (return (`|GetArrayItem` (`|MakeArray` (struct :`R` 1.0 :`B` 0.007499 :`A` 1.0) (struct :`R` 1.0 :`B` 0.007499 :`A` 1.0) (struct :`R` 1.0 :`B` 0.007499 :`A` 1.0) (struct :`R` 0.023153 :`G` 0.155926 :`A` 1.0) (struct :`R` 0.023153 :`G` 0.155926 :`A` 1.0) (struct :`R` 0.023153 :`G` 0.155926 :`A` 1.0) (struct :`R` 0.151042 :`B` 0.133611 :`A` 1.0) (struct :`G` 0.027321 :`B` 1.0 :`A` 1.0) (struct :`R` 1.0 :`G` 0.08022 :`A` 1.0) (struct :`G` 0.027321 :`B` 1.0 :`A` 1.0) (struct :`R` 1.0 :`G` 0.08022 :`A` 1.0) (struct :`G` 0.027321 :`B` 1.0 :`A` 1.0) (struct :`R` 1.0 :`G` 0.08022 :`A` 1.0) (struct :`G` 0.610496 :`B` 0.095307 :`A` 1.0) (struct :`R` 0.201556 :`G` 0.084376 :`B` 0.012286 :`A` 1.0) (struct :`R` 0.254152 :`G` 0.254152 :`B` 0.254152 :`A` 1.0) (struct :`R` 0.201556 :`G` 0.084376 :`B` 0.012286 :`A` 1.0) (struct :`R` 0.760525 :`G` 0.723055 :`A` 1.0) (struct :`R` 0.760525 :`G` 0.723055 :`A` 1.0) (struct :`R` 0.760525 :`G` 0.723055 :`A` 1.0) (struct :`R` 0.254152 :`G` 0.254152 :`B` 0.254152 :`A` 1.0) (struct :`R` 1.0 :`G` 0.08022 :`A` 1.0) (struct :`R` 0.760525 :`G` 0.723055 :`A` 1.0) (struct :`R` 0.201556 :`G` 0.084376 :`B` 0.012286 :`A` 1.0) :!type "LinearColor Structure") _returnvalue))
    (else
      (bind _output_get (set `self.Train Letter` (`|GetArrayItem` _array (`KismetMathLibrary.RandomIntegerInRange` 0 (`KismetArrayLibrary.Array_LastIndex` _array)))))
      (bind _output (`self.GetTrainColorByLetter` _output_get))
      (return _output))))

(fn `MakeArrayOfLights`
  (returns (Array :type "Array of PointLightComponent Object Reference"))
  (return (`|MakeArray` (`self.LightEmitter8`) (`self.LightEmitter1`) (`self.LightEmitter2`) (`self.LightEmitter3`) (`self.LightEmitter4`) (`self.LightEmitter5`) (`self.LightEmitter6`) (`self.LightEmitter7`) (`self.LightEmitter`) (`self.LightEmitter9`) (`self.LightEmitter10`) (`self.LightEmitter11`) (`self.LightEmitter12`) (`self.LightEmitter13`) (`self.LightEmitter15`) (`self.LightEmitter14`))))

(fn `MakeTrainHeadlightsColor`
  (returns (Array :type "Array of LinearColor Structure"))
  (return (`|MakeArray` (make `LinearColor` :`R` 255.0 :`G` 255.0 :`B` 255.0) (make `LinearColor` :`R` 255.0))))

(fn `MakeTrainLights`
  (returns (`Black Lights` :type "Array of PointLightComponent Object Reference") (`Front Lights` :type "Array of PointLightComponent Object Reference") (`Destination Text` :type "Array of TextRenderComponent Object Reference") (`Train Car ID` :type "Array of TextRenderComponent Object Reference"))
  (return (`|MakeArray` (`self.HeadLightBLB`) (`self.HeadLightBLT`) (`self.HeadLightBRB`) (`self.HeadLightBRT`)) (`|MakeArray` (`self.HeadLightFLB`) (`self.HeadLightFLT`) (`self.HeadLightFRB`) (`self.HeadLightFRT`)) (`|MakeArray` (`self.DestinationText_BR`) (`self.DestinationText_FR`) (`self.DestinationText_BL`) (`self.DestinationText_FL`)) (`|MakeArray` (`self.TrainID_BL`) (`self.TrainID_FL`) (`self.TrainID_FR`) (`self.TrainID_BR`))))

(fn `SetInvisibleTrainSparks`
  (params (bNewVisibility :type Boolean))
  (`SceneComponent.SetVisibility` (`self.sparks`) bNewVisibility true))

(fn `SetTrainColor`
  (bind _output (`self.GetTrainColorByLetter` (`KismetStringLibrary.ToUpper` (`self.Train Letter`))))
  (for _array_element (`|MakeArray` (`self.TrainColor_F`) (`self.TrainColor_FR`) (`self.TrainColor_BR`) (`self.TrainColor_FL`) (`self.TrainColor_BL`) (`self.TrainColor_B`))
    (bind _returnvalue (`PrimitiveComponent.CreateDynamicMaterialInstance` _array_element 0 "/Game/Texture_Model/Materials/TrainColors/M_OneColorToRuleThemAll.M_OneColorToRuleThemAll" "None"))
    (`MaterialInstanceDynamic.SetVectorParameterValue` _returnvalue "Changable Color" _output))
  (return))

(fn `SetTrainDestination`
  (params (Array :type "Array of TextRenderComponent Object Reference"))
  (for _array_element Array
    (bind _returnvalue (`GameplayStatics.GetCurrentLevelName` true))
    (`TextRenderComponent.K2_SetText` _array_element (`KismetTextLibrary.Conv_StringToText` _returnvalue))))

(fn `SetTrainLetter`
  (for _array_element (`|MakeArray` (`self.TrainSymbol_FL`) (`self.TrainSymbol_BL`) (`self.TrainSymbol_FR`) (`self.TrainSymbol_F`) (`self.TrainSymbol_B`) (`self.TrainSymbolTop_F`) (`self.TrainSymbolTop_B`) (`self.TrainSymbol_BR`))
    (`TextRenderComponent.K2_SetText` _array_element (`KismetTextLibrary.Conv_StringToText` (`KismetStringLibrary.ToUpper` (`self.Train Letter`)))))
  (return))

(fn `SetTrainLights`
  (params (`Front Lights` :type "Array of PointLightComponent Object Reference") (`Back Lights` :type "Array of PointLightComponent Object Reference") (`Is Flipped` :type Boolean) (`Is Head` :type Boolean))
  (bind _array (`self.MakeTrainHeadlightsColor`))
  (bind _output (`|GetArrayItem` _array))
  (bind _output_2 (`|GetArrayItem` _array 1))
  (for _array_element `Front Lights`
    (if `Is Flipped`
      (`LightComponent.SetLightColor` _array_element _output_2 true)
      (else
        (`LightComponent.SetLightColor` _array_element _output true)))
    (if `Is Head`
      (`LightComponent.SetIntensity` _array_element 10000.0)))
  (for _array_element_2 `Back Lights`
    (if `Is Flipped`
      (`LightComponent.SetLightColor` _array_element_2 _output true)
      (else
        (`LightComponent.SetLightColor` _array_element_2 _output_2 true)))
    (if `Is Head`
      (`LightComponent.SetIntensity` _array_element_2 10000.0))))

(fn `SetTrainUniqueID`
  (params (Array :type "Array of TextRenderComponent Object Reference"))
  (bind _output_get (set `self.TrainNumber` (`KismetMathLibrary.RandomIntegerInRange` 1000 9999)))
  (for _array_element Array
    (`TextRenderComponent.K2_SetText` _array_element (`KismetTextLibrary.Conv_IntToText` _output_get false false))))

(fn `Setup`
  (params (`Is Flipped` :type Boolean) (`Is Head` :type Boolean) (Velocity :type "Vector Structure") (`Train Letter` :type String) (VisibilitySparks :type Boolean))
  (bind (_black_lights _front_lights _destination_text _train_car_id) (`self.MakeTrainLights`))
  (set `self.IsFlipped` `Is Flipped`)
  (set `self.IsHead` `Is Head`)
  ;[1 1 1] set dynamic lights and text
  (set `self.InitialVelocity` Velocity)
  (set `self.Train Letter` `Train Letter`)
  (`self.SetTrainLights` _front_lights _black_lights `Is Flipped` `Is Head`)
  (`self.SetTrainDestination` _destination_text)
  (`self.SetTrainUniqueID` _train_car_id)
  (set `MovementComponent.Velocity` Velocity (`self.ProjectileMovement`))
  (`self.SetTrainColor`)
  (`self.SetTrainLetter`)
  (`self.SetInvisibleTrainSparks` VisibilitySparks))

(fn `SetVisibilityOfOtherWidgets`
  (params (InVisibility :type "ESlateVisibility Enum" :default "Visible"))
  (bind _foundwidgets (`WidgetBlueprintLibrary.GetAllWidgetsOfClass` "/Game/UI/InGame/InGameUI.InGameUI_C"))
  (`Widget.SetVisibility` _foundwidgets InVisibility))

(fn `UserConstructionScript`
  (`self.Setup` (`self.IsFlipped`) (`self.IsHead`) (`self.Velocity`) (`self.Train Letter`) (`self.SparkVisibility`)))