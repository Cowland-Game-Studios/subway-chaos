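; Test actor that detects a press-and-hold of the left mouse button, printing debug text.
; It enables input for player controller 0 on BeginPlay, then tracks press and release in the Held flag.
; Each press restarts a one-second retriggerable delay, after which StillHeld prints a message if the button is down.
; It contains no drag movement logic.
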(event `Key|LeftMouseButton` :consume false :overrideparent false
  (params (Key :type "Key Structure"))
  (:`Pressed`
    (`KismetSystemLibrary.PrintString` "p" true true (struct :`G` 0.66 :`B` 1.0 :`A` 1.0) 10.0)
    (set `self.Held` true)
    (`KismetSystemLibrary.RetriggerableDelay` 1.0)
    (`self.StillHeld`))
  (:`Released`
    (`KismetSystemLibrary.PrintString` "r" true true (struct :`G` 0.66 :`B` 1.0 :`A` 1.0) 10.0)
    (set `self.Held` false)))

(event `self.ReceiveBeginPlay`
  (`self.EnableInput` (`GameplayStatics.GetPlayerController` 0)))

(fn `StillHeld`
  (if (`self.Held`)
    (`KismetSystemLibrary.PrintString` "Hello")))

(fn `UserConstructionScript`)