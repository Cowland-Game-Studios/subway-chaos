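; Mouse-driven pick-up Blueprint that enables cursor, click and touch events on player 0 and drags a grabbed component around the world.
; GrabObject traces under the cursor and attaches the hit component to a PhysicsHandle, and ReleaseObject lets go.
; While holding, Tick sweeps the component by a scaled cursor projection onto the Z=0 plane, added to its location.
; The grab/release toggle and simulating-physics check are disconnected, so nothing here triggers a grab.
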(event `self.ReceiveBeginPlay`
  (bind _returnvalue (`GameplayStatics.GetPlayerController` 0))
  (set `PlayerController.bShowMouseCursor` true (`GameplayStatics.GetPlayerController` 0))
  (set `PlayerController.bEnableMouseOverEvents` true (`GameplayStatics.GetPlayerController` 0))
  (set `PlayerController.bEnableClickEvents` true (`GameplayStatics.GetPlayerController` 0))
  (set `PlayerController.bEnableTouchEvents` true _returnvalue)
  (`KismetArrayLibrary.Array_Append` (`PlayerController.ClickEventKeys` _returnvalue) (`|MakeArray` "RightMouseButton" :!type "Key Structure")))

(event `self.ReceiveTick`
  (params (DeltaSeconds :type "Float (single-precision)"))
  (bind _objectpickedup (`self.ObjectPickedUp`))
  (`/Engine/EditorBlueprintResources/StandardMacros.IsValid` _objectpickedup
    (:`Is Valid`
      (if (`self.holding`)
        (`SceneComponent.K2_SetWorldLocationAndRotation` _objectpickedup (+ (`SceneComponent.K2_GetComponentLocation` _objectpickedup) (`self.GetOver`)) (`SceneComponent.K2_GetComponentRotation` _objectpickedup) true false)))))

(fn `GetFacingDirection`
  (returns (ReturnValue :type "Vector Structure"))
  (return (`KismetMathLibrary.Vector_GetAbs` (- (`KismetMathLibrary.GetForwardVector` (`SceneComponent.K2_GetComponentRotation` (`self.DefaultSceneRoot`))) 1))))

(fn `GetOver`
  (returns (ReturnValue :type "Vector Structure"))
  (bind (_worldlocation _worlddirection) (`PlayerController.DeprojectMousePositionToWorld` (`GameplayStatics.GetPlayerController` 0)))
  (return (/ (+ _worldlocation (* (* _worlddirection (/ (.z _worldlocation) (.z _worlddirection))) -1.0)) 30)))

(fn `GrabObject`
  (bind (_hitresult _returnvalue) (`PlayerController.GetHitResultUnderCursorByChannel` (`GameplayStatics.GetPlayerController` 0) "TraceTypeQuery1" true))
  (if _returnvalue
    (`PhysicsHandleComponent.GrabComponentAtLocation` (`self.PhysicsHandle`) (`.HitComponent` (`GameplayStatics.BreakHitResult` _hitresult)) "None" (`SceneComponent.K2_GetComponentLocation` (`.HitComponent` (`GameplayStatics.BreakHitResult` _hitresult))))
    (set `self.holding` true)
    (`KismetSystemLibrary.PrintString` "Hello")
    (set `self.ObjectPickedUp` (`.HitComponent` (`GameplayStatics.BreakHitResult` _hitresult)))))

(fn `ReleaseObject`
  (`PhysicsHandleComponent.ReleaseComponent` (`self.PhysicsHandle`))
  (set `self.holding` false))

(fn `UserConstructionScript`)